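; Camera rig that exports cube capture frames to disk for GearVR stereoscopic rendering, one numbered image per eye.
; When tick export is enabled, it counts frames and, at the configured start frame, assigns render targets and enables every-frame capture, with the right eye capturing only in stereo.
; Later frames export each texture with a zero-padded frame number, and periodic garbage collection limits RAM-related crashes during the slow export.
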(event `self.ReceiveTick`
  (params (DeltaSeconds :type "Float (single-precision)"))
  (bind _capturecomponentcube (`self.CaptureComponentCube`))
  (bind _righteye (`self.RightEye`))
  (bind _returnvalue (`KismetTextLibrary.Conv_TextToString` (`KismetTextLibrary.Conv_IntToText` (`self.FrameNum`) false 5)))
  (if (`self.bExportOnTick`)
    (`|ExecutionSequence`
      (:`then_0`
        (if (== (`self.FrameNum`) (`self.FrameSkipUntilAfter`))
          ;[1 1 1] Turn up Capture Every Frame as we want to be capturing by next frame
          (`|ExecutionSequence`
            (:`then_0`
              (`/Engine/EditorBlueprintResources/StandardMacros.Gate` false :!label _label
                (:`Exit`
                  (set `SceneCaptureComponentCube.TextureTarget` (`self.LeftEyeTexture`) _capturecomponentcube)
                  (set `SceneCaptureComponent.bCaptureEveryFrame` true _capturecomponentcube)
                  (set `SceneCaptureComponentCube.TextureTarget` (`self.RightEyeTexture`) _righteye)
                  (set `SceneCaptureComponent.bCaptureEveryFrame` (`self.bStereo`) _righteye)
                  (goto _label :!via `Close`))))
            (:`then_1`
              (set `self.FrameNum` (+ (`self.FrameNum`) 1))))
          (elif (> (`self.FrameNum`) (`self.FrameSkipUntilAfter`))
            (`|ExecutionSequence`
              (:`then_0`
                (goto _label))
              (:`then_1`
                ;[1 1 1] Export render texture targets (very slow)
                (`StereoscopicRenderBlueprintLibrary.ExportObjectToPath` (`self.LeftEyeTexture`) (`self.ExportDirectory`) _returnvalue)
                (`|ExecutionSequence`
                  (:`then_0`
                    (if (`self.bStereo`)
                      (`StereoscopicRenderBlueprintLibrary.ExportObjectToPath` (`self.RightEyeTexture`) (`self.ExportDirectory`) _returnvalue)))
                  (:`then_1`
                    ;[1 1 1] Collect garbage after set number of frames (Helps prevent crashing because of overloading RAM)
                    (if (> (- (`self.FrameNum`) (`self.LastGarbageCollectFrame`)) (`self.GarbageCollectAfterNumFrames`))
                      (`KismetSystemLibrary.CollectGarbage`)
                      (set `self.LastGarbageCollectFrame` (`self.FrameNum`))
                      (`KismetSystemLibrary.PrintString` "Garbage Collected!!!!" false true (struct :`G` 1.0 :`B` 0.189364 :`A` 1.0))))))
              (:`then_2`
                ;[1 1 1] Update frame number
                (set `self.FrameNum` (+ (`self.FrameNum`) 1) :!label _label_2)))
            (else
              (goto _label_2)))))
      (:`then_1`
        ;[1 1 1] Account for Garbage Collection if skipping frames
        (`/Engine/EditorBlueprintResources/StandardMacros.DoOnce` false
          (:`Completed`
            (set `self.LastGarbageCollectFrame` (`self.FrameSkipUntilAfter`))))))))

(fn `UserConstructionScript`)